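; Enemy Blueprint with 100 HP that reacts to damage and to overlapping actors implementing DamageInterface.
; At zero HP it notifies ShooterGameMode through DecreaseEnemy, then calls DestroyActor on the cast game mode rather than itself.
; Overlap stores the Hero and sets a named timer targeting that Hero, though the handler sending DecreaseHpMessage, with zero damage, lives on the enemy.
; End overlap clears the timer on the enemy.
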(event Custom|Decread%20Hero%20Hp
  (Class|DamageInterface|DecreaseHp(Message) (Variables|Default|GetHero) 0.0))

(event EventBeginPlay
  (Variables|Default|SetHp 1e+02))

(event EventDecreaseHP
  (params (Amount :type Float%20%28single-precision%29))
  (bind _output_get (Variables|Default|SetHp (- (Variables|Default|GetHp) Amount)))
  (if (<= _output_get 0.0)
    (bind _asshooter_game_mode (Utilities|Casting|CastToShooterGameMode (Game|GetGameMode)))
    (Default|DecreaseEnemy _asshooter_game_mode)
    (bind _asshooter_game_mode_2 (Utilities|Casting|CastToShooterGameMode (Game|GetGameMode)))
    (Actor|DestroyActor _asshooter_game_mode_2)))

(event Collision|EventActorBeginOverlap
  (params (OtherActor :type Actor%20Object%20Reference))
  (if (Utilities|DoesObjectImplementInterface OtherActor "/Game/Interface/DamageInterface.DamageInterface_C")
    (bind _output_get (Variables|Default|SetHero OtherActor))
    (Utilities|Time|SetTimerbyFunctionName _output_get "Decread Hero Hp" 0.33)))

(event Collision|EventActorEndOverlap
  (params (OtherActor :type Actor%20Object%20Reference))
  (if (== OtherActor (Variables|Default|GetHero))
    (Utilities|Time|ClearTimerbyFunctionName 0 "Decread Hero Hp")))

(fn ConstructionScript)