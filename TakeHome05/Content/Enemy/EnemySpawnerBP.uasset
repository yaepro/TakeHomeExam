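; Enemy spawner that spawns EnemyBP pawns at random points inside its SpawnArea box.
; On BeginPlay it checks for ShooterGameMode and starts a looping two-second timer on SpawnEnemy.
; SpawnEnemy spawns only when the game mode's NumberEnemies is zero or less, then calls IncreaseEnemy.
; The GameMode variable it reads is set to None after the cast, rather than to the cast result.
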(event Custom|SpawnEnemy
  (bind _spawn_area (Variables|Default|GetSpawn%20Area))
  (bind _gamemode (Variables|Default|GetGameMode))
  (if (<= (Variables|/Game/ShooterGameMode.ShooterGameMode_C|GetNumberEnemies _gamemode) 0)
    (AI|SpawnAIFromClass "/Game/Enemy/EnemyBP.EnemyBP_C" 0 (Math|Random|RandomPointinBoundingBox (Transformation|GetWorldLocation _spawn_area) (Components|Box|GetScaledBoxExtent _spawn_area)) "0, 0, 0" false)
    (Default|IncreaseEnemy _gamemode)))

(event EventBeginPlay
  (Utilities|Casting|CastToShooterGameMode (Game|GetGameMode))
  (Variables|Default|SetGameMode 0)
  (Utilities|Time|SetTimerbyFunctionName 0 "SpawnEnemy" 2.0 true))

(fn ConstructionScript)