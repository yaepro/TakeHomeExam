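; HeroBP is the player hero Blueprint that moves, turns and fires an attached gun.
; On BeginPlay it spawns a GunBP, stores it as Gun and snaps it to the mesh's GunPoint socket.
; The bullet trigger input calls Fire on that gun.
; Move axes push along fixed world X and Y regardless of facing, while the turn axis adds scaled local yaw each update without delta-time scaling.
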(event EventBeginPlay
  (bind _returnvalue (Game|SpawnActorfromClass "/Game/Gun/GunBP.GunBP_C" (Transformation|GetWorldTransform (Variables|Character|GetMesh)) "Undefined" 0 0))
  (bind _output_get (Variables|Default|SetGun _returnvalue))
  (Transformation|AttachComponentToComponent _output_get (Variables|Character|GetMesh) "GunPoint" "SnapToTarget" "SnapToTarget" "KeepRelative" true))

(event Input|ActionEvents|InputActionTriggerBullet
  (params (Key :type Key%20Structure :default "AnyKey"))
  (:Pressed
    (Default|Fire (Variables|Default|GetGun))))

(event Input|AxisEvents|InputAxisMoveForward
  (params (AxisValue :type Float%20%28single-precision%29))
  (Pawn|Input|AddMovementInput "1.000000, 0, 0" AxisValue false))

(event Input|AxisEvents|InputAxisTurnRight
  (params (AxisValue :type Float%20%28single-precision%29))
  (Transformation|AddActorLocalRotation (Math|Rotator|MakeRotator 0.0 0.0 (* AxisValue 3.0)) false false))

(event Input|AxisEvents|InputAxisMoveRight
  (params (AxisValue :type Float%20%28single-precision%29))
  (Pawn|Input|AddMovementInput "0,1.000000, 0" AxisValue false))

(fn ConstructionScript)